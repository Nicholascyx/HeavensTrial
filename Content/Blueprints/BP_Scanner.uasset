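; BP_Scanner is an expanding scanner actor that displaces the owning VR pawn when the two overlap.
; Tick grows the actor's scale without limit at a rate set by ScanSpeed.
; BeginPlay caches the owner as a VRPawn.
; On overlapping that pawn, MoveComponentTo moves its capsule over a short time to a relative location built from the negated, scaled forward vector, without adding the current position.
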(event `self.ReceiveTick`
  (params (DeltaSeconds :type "Float (single-precision)"))
  (`self.SetActorScale3D` (+ (* DeltaSeconds (`self.Scan Speed`)) (`self.GetActorScale3D`))))

(event `self.ReceiveBeginPlay`
  (bind _asvrpawn (cast `/Game/Blueprints/VRPawn` (`self.GetOwner`)))
  (set `self.Player` _asvrpawn))

(event `self.ReceiveActorBeginOverlap`
  (params (OtherActor :type "Actor Object Reference"))
  (if (== OtherActor (`self.Player`))
    (`KismetSystemLibrary.MoveComponentTo` (`Character.CapsuleComponent` (`self.Player`)) (* (`SceneComponent.GetForwardVector` (`Character.CapsuleComponent` (`self.Player`))) -10.0) (struct) false false 0.3)))

(fn `UserConstructionScript`)