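; BP_GrappleAnchor is an interactable grapple point that the player hooks onto and releases through interact begin and end events.
; Grappling plays a web-shooting sound at the player, sets the player's grappling flag and updates grapple visibility.
; Releasing clears the grappling and length-set flags, updates visibility and calls the player's launch at the end of the grapple.
; The anchor only toggles state on the player and returns itself through GetActor.
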(event `/Game/BlueprintInterface/BPI_Interaction.InteractBegin`
  (params (Player :type "/Game/Blueprints/VRPawn Object Reference"))
  (`self.Grapple` Player))

(event `/Game/BlueprintInterface/BPI_Interaction.InteractEnd`
  (params (Player :type "/Game/Blueprints/VRPawn Object Reference"))
  (`self.Ungrapple` Player))

(fn `GetActor`
  (returns (Actor :type "Actor Object Reference"))
  (return self))

(fn `Grapple`
  (params (Player :type "/Game/Blueprints/VRPawn Object Reference"))
  (`GameplayStatics.PlaySoundAtLocation` "/Game/Audio/SoundWaves/Effect/SW_WebShooting.SW_WebShooting" (`self.K2_GetActorLocation` Player) (struct) 1.0 1.0 0.4 null null null null)
  (bind _output_get (set `/Game/Blueprints/VRPawn.IsGrappling` true Player))
  (`/Game/Blueprints/VRPawn.HandleGrappleVisibility` Player _output_get))

(fn `Ungrapple`
  (params (Player :type "/Game/Blueprints/VRPawn Object Reference"))
  (bind _output_get (set `/Game/Blueprints/VRPawn.IsGrappling` false Player))
  (`/Game/Blueprints/VRPawn.HandleGrappleVisibility` Player _output_get)
  (set `/Game/Blueprints/VRPawn.IsGrappleLengthSet` false Player)
  (`/Game/Blueprints/VRPawn.LaunchAtGrappleEnd` Player))

(fn `UserConstructionScript`)