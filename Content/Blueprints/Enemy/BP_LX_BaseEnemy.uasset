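; BP_LX_BaseEnemy is a base enemy that shoots projectiles at a VR pawn it perceives.
; An AIPerception update on a VRPawn sets IsTracking and, on a successful sense, stores the pawn and starts a looping ShootPlayer timer at ShootDelay.
; ShootPlayer spawns BP_LX_BaseProjectile at the Arrow transform, passing ProjectileSpeed and the tracked pawn as target.
; Losing the pawn only clears IsTracking; nothing here stops the timer.
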(event `self.AIPerception.OnTargetPerceptionUpdated`
  (params (Actor :type "Actor Object Reference") (Stimulus :type "AIStimulus Structure"))
  ; Track pawn, assuming pawn is outside view range on spawn
  (bind _asvrpawn (cast `/Game/Blueprints/VRPawn` Actor))
  (bind _output_get (set `self.IsTracking` (`.bSuccessfullySensed` (break `AIStimulus` Stimulus))))
  (if _output_get
    (set `self.CurrentTrackedPawn` _asvrpawn)
    (`KismetSystemLibrary.K2_SetTimer` null "ShootPlayer" (`self.ShootDelay`) true)))

(fn `ShootPlayer`
  (`|SpawnActorFromClass` "/Game/Blueprints/Enemy/BP_LX_BaseProjectile.BP_LX_BaseProjectile_C" (`SceneComponent.K2_GetComponentToWorld` (`self.Arrow`)) "Undefined" "MultiplyWithRoot" self (`self.ProjectileSpeed`) (`self.CurrentTrackedPawn`) null))

(fn `UserConstructionScript`)