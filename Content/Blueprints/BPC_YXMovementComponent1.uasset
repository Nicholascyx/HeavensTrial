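; Actor component for a VRPawn that turns vertical arm swinging into faster walking, caching its owning pawn on BeginPlay.
; Each tick, when both motion controller grips' absolute Z velocities reach SwingBoundary, it adds them to Speed, doubles the sum and clamps it.
; Speed decays linearly down to about the clamp minimum, driving the pawn's MaxWalkSpeed as it falls.
; It only adjusts the speed limit and adds no movement input.
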(event `self.ReceiveBeginPlay`
  (bind _asvrpawn (cast `/Game/Blueprints/VRPawn` (`self.GetOwner`)))
  (set `self.Player` _asvrpawn))

(event `self.ReceiveTick`
  (params (DeltaSeconds :type "Float (single-precision)"))
  (bind _player (`self.Player`))
  (bind _swingboundary (`self.SwingBoundary`))
  (bind _returnvalue (`KismetMathLibrary.Abs` (.z (`MotionControllerComponent.GetLinearVelocity` (`/Game/Blueprints/VRPawn.MotionControllerRightGrip` _player)))))
  (bind _returnvalue_2 (`KismetMathLibrary.Abs` (.z (`MotionControllerComponent.GetLinearVelocity` (`/Game/Blueprints/VRPawn.MotionControllerLeftGrip` _player)))))
  (`|ExecutionSequence`
    (:`then_0`
      (if (>= (`self.Speed`) 150.0)
        (set `self.Speed` (- (`self.Speed`) (* DeltaSeconds 300.0)))
        (set `CharacterMovementComponent.MaxWalkSpeed` (`self.Speed`) (`Character.CharacterMovement` (`self.Player`)))))
    (:`then_1`
      (if (and (>= _returnvalue_2 _swingboundary) (>= _returnvalue _swingboundary))
        (set `self.Speed` (`KismetMathLibrary.FClamp` (* (+ _returnvalue_2 _returnvalue (`self.Speed`)) 2.0) 150.0 600.0))))))