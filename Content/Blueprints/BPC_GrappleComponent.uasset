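; Actor component that gives the VRPawn grapple swing and hook movement toward its interaction impact point, driven by external calls.
; HandleSwingMovement locks rope length, snaps the pawn back within it, gives a grounded initial push, then adds tangential and velocity-projected radial forces.
; Hook movement applies one strong pull force, and release launches along velocity.
; Helpers control the Grapple cable's visibility and endpoint; state lives on the pawn.
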(event `self.ReceiveBeginPlay`
  (bind _asvrpawn (cast `/Game/Blueprints/VRPawn` (`self.GetOwner`)))
  (set `self.Player` _asvrpawn))

(fn `ApplyDampingTangentialForce`
  ; Applies the opposite force to oppose the tangential force
  (`CharacterMovementComponent.AddForce` (`Character.CharacterMovement` (`self.Player`)) (`Actor.GetVelocity` (`self.Player`))))

(fn `ApplyRadialForce`
  ;[0.3854 0.3854 0.3854 0.5] Apply force along the grapple rope component
  (bind _returnvalue (`self.GetGrappleForce`))
  (`CharacterMovementComponent.AddForce` (`Character.CharacterMovement` (`self.Player`)) _returnvalue))

(fn `ApplySwingForces`
  ; Applies all the forces during the swing
  (`self.ApplyTangentialForce`)
  (`self.ApplyRadialForce`))

(fn `ApplyTangentialForce`
  ;[0.2969 0.2969 0.2969 0.5] Apply force along the velocity component
  (`CharacterMovementComponent.AddForce` (`Character.CharacterMovement` (`self.Player`)) (* (`KismetMathLibrary.Normal` (`Actor.GetVelocity` (`self.Player`))) 2.0)))

(fn `FixGrappleLength`
  (bind _player (`self.Player`))
  (bind _interactionimpactpoint (`/Game/Blueprints/VRPawn.InteractionImpactPoint` _player))
  (bind _currentgrapplelength (`/Game/Blueprints/VRPawn.CurrentGrappleLength` _player))
  (bind _returnvalue (- _interactionimpactpoint (`Actor.K2_GetActorLocation` _player)))
  ; Fixes the grapple component length to prevent the player from exceeding the maximum position they should be
  (if (> (`KismetMathLibrary.VSize` _returnvalue) _currentgrapplelength)
    (`Actor.K2_SetActorLocation` _player (- _interactionimpactpoint (* (`KismetMathLibrary.Normal` _returnvalue) _currentgrapplelength)) false false)))

(fn `GetGrappleForce`
  (returns (ReturnValue :type "Vector Structure"))
  (bind _player (`self.Player`))
  (bind _returnvalue (- (`/Game/Blueprints/VRPawn.InteractionImpactPoint` _player) (`Actor.K2_GetActorLocation` _player)))
  ; Returns the force along the grapple component to pull the player towards the swing point
  (return (* (* (`KismetMathLibrary.Normal` _returnvalue) (`KismetMathLibrary.Dot_VectorVector` (`Actor.GetVelocity` _player) _returnvalue)) -0.5)))

(fn `GetInitialPushForce`
  (returns (ReturnValue :type "Vector Structure"))
  (bind _player (`self.Player`))
  ; Returns the force to push the player at the beginning of the swing motion
  (if (`NavMovementComponent.IsMovingOnGround` (`Character.CharacterMovement` _player))
    (return (* (`KismetMathLibrary.Normal` (- (`/Game/Blueprints/VRPawn.InteractionImpactPoint` _player) (`Actor.K2_GetActorLocation` _player))) 20.0))
    (else
      (return (0.0 0.0 0.0)))))

(fn `HandleGrappleAttach`
  (bind _player (`self.Player`))
  (bind _grapple (`/Game/Blueprints/VRPawn.Grapple` _player))
  ;[0.2917 0.2917 0.2917 0.5] Handles the attachment of the grapple to the interaction impact point
  (set `CableComponent.EndLocation` (`KismetMathLibrary.InverseTransformLocation` (`SceneComponent.K2_GetComponentToWorld` _grapple) (`/Game/Blueprints/VRPawn.InteractionImpactPoint` _player)) _grapple))

(fn `HandleGrappleVisibility`
  (params (IsVisible :type Boolean))
  ;[0.2917 0.2917 0.2917 0.5] Sets the visibility of the grapple component
  (`SceneComponent.SetVisibility` (`/Game/Blueprints/VRPawn.Grapple` (`self.Player`)) IsVisible false))

(fn `HandleHookMovement`
  (bind _player (`self.Player`))
  (bind _charactermovement (`Character.CharacterMovement` _player))
  ; Handles the player movement when hooking towards the interaction impact point
  (set `CharacterMovementComponent.GravityScale` 0.0 _charactermovement)
  (`CharacterMovementComponent.AddForce` _charactermovement (* (`KismetMathLibrary.Normal` (- (`/Game/Blueprints/VRPawn.InteractionImpactPoint` _player) (`Actor.K2_GetActorLocation` _player))) 781250.0))
  (set `CharacterMovementComponent.GravityScale` 4.0 _charactermovement))

(fn `HandleSwingMovement`
  (bind _player (`self.Player`))
  ;[0.2917 0.2917 0.2917 0.5] Handles the player's movement at the start, end and during the swinging motion and should be the main function to call
  (if (not (`/Game/Blueprints/VRPawn.IsGrappleLengthSet` _player))
    (`self.SetCurrentGrappleLength`)
    (set `/Game/Blueprints/VRPawn.IsGrappleLengthSet` true _player))
  (`self.FixGrappleLength`)
  (if (not (`/Game/Blueprints/VRPawn.IsInitialPushed` _player))
    (`self.InitialPushPlayer`))
  (`self.ApplySwingForces`)
  (set `CharacterMovementComponent.AirControl` 0.5 (`Character.CharacterMovement` _player))
  (`KismetSystemLibrary.PrintString` (`KismetStringLibrary.Conv_DoubleToString` (`CableComponent.CableLength` (`/Game/Blueprints/VRPawn.Grapple` (`self.Player`))))))

(fn `InitialPushPlayer`
  (bind _player (`self.Player`))
  ; Pushes the player at the very beginning of the swing motion
  (bind _returnvalue (`self.GetInitialPushForce`))
  (`CharacterMovementComponent.AddForce` (`Character.CharacterMovement` _player) _returnvalue)
  (set `/Game/Blueprints/VRPawn.IsInitialPushed` true _player))

(fn `LaunchAtGrappleEnd`
  (bind _player (`self.Player`))
  ;[0.401 0.401 0.401 0.5] Launches the player when releasing the grapple
  (`CharacterMovementComponent.AddForce` (`Character.CharacterMovement` _player) (* (`Actor.GetVelocity` _player) 200.0)))

(fn `SetCurrentGrappleLength`
  (bind _player (`self.Player`))
  ; Sets the grapple component length to be fixed to the length between the player and the interaction impact point
  (bind _output_get (set `/Game/Blueprints/VRPawn.CurrentGrappleLength` (`KismetMathLibrary.VSize` (- (`/Game/Blueprints/VRPawn.InteractionImpactPoint` _player) (`Actor.K2_GetActorLocation` _player))) _player))
  (set `CableComponent.CableLength` _output_get (`/Game/Blueprints/VRPawn.Grapple` (`self.Player`))))