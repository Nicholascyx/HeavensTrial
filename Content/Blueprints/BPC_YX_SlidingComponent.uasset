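; BPC_YX_SlidingComponent is a component for a VRPawn owner, meant to trigger a slide from hand motion, but its YXSlide event is empty and the logic is unconnected.
; That logic samples both motion controller grips over a brief delay and checks for fast vertical movement of both hands.
; A match calls the pawn's slide-down, boosts walk speed for a second, then calls slide-up and lowers it.
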(event `YXSlide`)